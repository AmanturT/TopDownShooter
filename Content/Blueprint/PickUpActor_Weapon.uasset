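; Weapon pickup actor that adds a weapon to a character's inventory when the character overlaps it.
; It overrides the OverlapCharacter event, runs the parent logic, then appends its WeaponSlotInfo to the WeaponSlots array of the passed InventoryComponent.
; The construction script only calls the parent, and the BeginPlay, Tick and ActorBeginOverlap nodes are disabled.
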(event `self.OverlapCharacter`
  (params (InventoryComponent :type "InventoryComponent Object Reference"))
  (`parent.OverlapCharacter` InventoryComponent)
  (`KismetArrayLibrary.Array_Add` (`InventoryComponent.WeaponSlots` InventoryComponent) (`self.WeaponSlotInfo`)))

(fn `UserConstructionScript`
  (`parent.UserConstructionScript`))