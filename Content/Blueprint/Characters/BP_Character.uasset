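; Top-down shooter player character that manages the camera, HUD, inventory screen, damage effects and death/respawn handling.
; The camera zooms in timer steps, shifts toward the cursor while aiming, and swaps materials on view-blocking objects to fade them.
; Weapon, health, shield and stamina events refresh widgets, with blood or spark effects on damage.
; Input sets sprint, walk and aim states, toggles the code-built inventory grid and night vision, and triggers test damage.
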(event `InputAxis|MouseWheel`
  (params (AxisValue :type "Float (single-precision)"))
  ;[1 0.8667 0.2667] Плавное отдаление/приближение камеры
  (if (`self.SlideWithSmooth`)
    (`self.CameraSldeFunction` AxisValue)))

(event `self.ReceiveTick`
  (params (DeltaSeconds :type "Float (single-precision)"))
  (bind _cameraboom (`self.CameraBoom`))
  (bind _cameraboom_2 (`self.CameraBoom`))
  (bind _topdowncameracomponent (`self.TopDownCameraComponent`))
  (bind _returnvalue (`SceneComponent.K2_GetComponentLocation` (`self.CapsuleComponent`)))
  (bind (_returnvalue_x _returnvalue_y _returnvalue_z) (`KismetMathLibrary.BreakVector` (`SceneComponent.K2_GetComponentLocation` _cameraboom)))
  (`|ExecutionSequence`
    (:`then_1`
      ;[0.3725 0.3961 1] Aiming
      (bind _returnvalue_2 (`self.GetCursorToWorld`))
      (set `self.ClampedCameraHeight` (`KismetMathLibrary.MapRangeClamped` (`SpringArmComponent.TargetArmLength` (`self.CameraBoom`)) (`self.CameraHeightMin`) (`self.CameraHeightMax`) 0.5 1.0))
      (bind _returnvalue_3 (`SceneComponent.K2_GetComponentLocation` _returnvalue_2))
      (set `self.DistanceCameraBoomChar` (`KismetMathLibrary.VSizeXY` (- _returnvalue _returnvalue_3)))
      (if (or (`|EnumEquality` (`self.CurrentMovementState`) "Aim_State") (`|EnumEquality` (`self.CurrentMovementState`) "WalkAim_State"))
        (if (< (* (`self.ClampedCameraHeight`) (`self.fMinClampDistanceLogicMouseCursorStart`)) (`self.DistanceCameraBoomChar`))
          (if (not (> (`KismetMathLibrary.VSize2D` (`KismetMathLibrary.Conv_VectorToVector2D` (- (`SceneComponent.K2_GetComponentLocation` (`self.CameraBoom`)) _returnvalue))) (* (`self.ClampedCameraHeight`) (`self.fMaxClampDistanceLogicMouseCursorStart`))))
            (bind (_x _y) (`KismetMathLibrary.BreakVector2D` (* (`KismetMathLibrary.Normal2D` (`KismetMathLibrary.Conv_VectorToVector2D` (`KismetMathLibrary.GetForwardVector` (`KismetMathLibrary.FindLookAtRotation` _returnvalue _returnvalue_3)))) (`self.fSpeedChangeLocationCameraToCursor`))))
            (`SceneComponent.K2_SetWorldLocation` _cameraboom (`KismetMathLibrary.MakeVector` (+ _returnvalue_x _x) (+ _returnvalue_y _y) _returnvalue_z) false false))
          (else
            (`SceneComponent.K2_SetWorldLocation` _cameraboom_2 (`KismetMathLibrary.VInterpTo` (`SceneComponent.K2_GetComponentLocation` _cameraboom_2) (`SceneComponent.K2_GetComponentLocation` (`self.CapsuleComponent`)) DeltaSeconds (`self.fSpeedReturnCameraDefaltPosition`)) false false :!label _label)))
        (else
          (goto _label))))
    (:`then_2`
      ;[1 0.8667 0.2667] Прозрачные стены(Если перекрывает поле видимости игрока)
      (bind (_outhit _returnvalue_4) (`KismetSystemLibrary.LineTraceSingle` (`SceneComponent.K2_GetComponentLocation` _topdowncameracomponent) (+ (`SceneComponent.GetForwardVector` _topdowncameracomponent) (`self.K2_GetActorLocation`)) "TraceTypeQuery1"))
      (if _returnvalue_4
        (`|ExecutionSequence`
          (:`then_0`
            (`/Engine/EditorBlueprintResources/StandardMacros.DoOnce` false :!label _label_2
              (:`Completed`
                (bind (_bblockinghit _binitialoverlap _time _distance _location _impactpoint _normal _impactnormal _physmat _hitactor _hitcomponent) (`GameplayStatics.BreakHitResult` _outhit))
                (set `self.PrimaryMaterial` (`PrimitiveComponent.GetMaterial` _hitcomponent 0)))))
          (:`then_1`
            (bind _output_get (set `self.Hit Component` _hitcomponent))
            (`PrimitiveComponent.SetMaterial` _output_get 0 "/Game/Blueprint/Characters/M_Fade.M_Fade")))
        (else
          (`/Engine/EditorBlueprintResources/StandardMacros.IsValid` _output_get
            (:`Is Valid`
              (`PrimitiveComponent.SetMaterial` (`self.Hit Component`) 0 (`self.PrimaryMaterial`))
              (goto _label_2 :!via `Reset`))))))))

(event `Key|H`
  (params (Key :type "Key Structure"))
  ;[1 0.3569 0.8471] Death TEST
  (:`Pressed`
    (`TPSHealthComponent.ChangeHealthValue` (`self.CharHealthComponent`) -50.0)))

(event `Key|Z`
  (params (Key :type "Key Structure")))

(event `self.CharDead_BP`
  (bind _asbp_game_mode_base (cast `/Game/Blueprint/Game/BP_GameModeBase` (`GameplayStatics.GetGameMode`)))
  (bind (_bissuccess _currentlives) (`/Game/Blueprint/Game/BP_GameModeBase.TryToRespawn` _asbp_game_mode_base))
  (if _bissuccess
    (bind _returnvalue (`self.GetCurrentWeapon`))
    (`self.SetLifeSpan` _returnvalue 20.0)
    (`self.SetLifeSpan` 20.0)
    (`/Game/Blueprint/UI/UI_StatsWidget.ChangeLivesWidget` (`self.StatsWidget`) _currentlives)
    (`Widget.RemoveFromParent` (`self.HealthWidget`))
    (`Widget.RemoveFromParent` (`self.StaminaWidget`))
    (`Widget.RemoveFromParent` (`self.StatsWidget`))
    (else
      (bind _returnvalue_2 (`|CreateWidget` "/Game/Blueprint/UI/UI_DeathScreen.UI_DeathScreen_C"))
      (`UserWidget.AddToViewport` _returnvalue_2 0))))

(event `self.WeaponReloadStart_BP`
  (params (Anim :type "AnimMontage Object Reference"))
  ;[0.3725 0.3961 1] MagazineDrop
  (`|PlayMontage` (`self.Mesh`) Anim
    (:`then`
      (bind _returnvalue (`self.GetCurrentWeapon`))
      (set `WeaponDefault.BlockReloading` true _returnvalue)
      (`WeaponDefault.SpawnMagazineDrop` _returnvalue)
      (`self.PlayReloadinAnim`))
    (:`OnCompleted`
      (set `WeaponDefault.BlockReloading` false _returnvalue))))

(event `self.ReceiveBeginPlay`
  ;[0.3725 0.3961 1] Виджет оружия и патронов(Надо переделать..)
  ;;[0.3725 0.3961 1] Создание виджетов и изменение иконок при свитчеоружия
  (`|ExecutionSequence`
    (:`then_0`
      (bind _returnvalue (`|CreateWidget` "/Game/Blueprint/UI/Inventory/WeaponWidget.WeaponWidget_C"))
      (`UserWidget.AddToViewport` _returnvalue 0)
      (bind _returnvalue_2 (`|CreateWidget` "/Game/Blueprint/UI/Inventory/ProjectileWidget.ProjectileWidget_C"))
      (`UserWidget.AddToViewport` _returnvalue_2 0)
      (bind _currentround (`/Game/Blueprint/UI/Inventory/ProjectileWidget.CurrentRound` _returnvalue_2))
      (`self.ChangeAmmoWidget` _currentround _returnvalue_2)
      (set `self.ProjectileWidget` _returnvalue_2))
    (:`then_1`
      (bind _returnvalue_3 (`self.GetCurrentWeapon` :!label _label_3))
      (`/Engine/EditorBlueprintResources/StandardMacros.IsValid` _returnvalue_3
        (:`Is Valid`
          (bind (_weaponsetting_weaponclass _weaponsetting_rateoffire _weaponsetting_reloadtime _weaponsetting_maxround _weaponsetting_numberprojectilebyshot _weaponsetting_dispersionweapon _weaponsetting_soundfireweapon _weaponsetting_soundreloadweapon _weaponsetting_effectfireweapon _weaponsetting_projectilesetting _weaponsetting_weapondamage _weaponsetting_distacnetrace _weaponsetting_decalonhit _weaponsetting_animweaponinfo _weaponsetting_magazinedrop _weaponsetting_shellbullets _weaponsetting_impusleofshelldrop _weaponsetting_switchtimetoweapon _weaponsetting_weaponicon _weaponsetting_projectileicon) (break `WeaponInfo` (`WeaponDefault.WeaponSetting` _returnvalue_3)))
          (`Image.SetBrushFromTexture` (`/Game/Blueprint/UI/Inventory/WeaponWidget.WeaponImage` _returnvalue) _weaponsetting_weaponicon false)
          (set `self.CurrentWeaponReloadingTime` _weaponsetting_reloadtime)
          (`Image.SetBrushFromTexture` (`/Game/Blueprint/UI/Inventory/ProjectileWidget.ProjectileImage` _returnvalue_2) _weaponsetting_projectileicon false)
          ;;[0.3725 0.3961 1] Изменение кол-во патронов при свитче и стрельбе и перезарядки
          (`self.ChangeAmmoWidget` _currentround _returnvalue_2))))
    (:`then_2`
      (`self.HealthWidgetCreating`))
    (:`then_3`
      (add `self.OnStaminaChanged` (delegate `OnStaminaChanged_Event_0`)))))

(event `self.WeaponReloadEnd_BP`
  (params (bIsSuccess :type Boolean))
  ;[0.3725 0.3961 1] Виджет оружия и патронов(Надо переделать..)
  ;;[0.3725 0.3961 1] Изменение кол-во патронов при свитче и стрельбе и перезарядки
  (if bIsSuccess
    (`self.ChangeAmmoWidget` (`/Game/Blueprint/UI/Inventory/ProjectileWidget.CurrentRound` (stale `self.ReceiveBeginPlay` _returnvalue_2)) (stale `self.ReceiveBeginPlay` _returnvalue_2) :!label _label_4)))

(event `self.WeaponFireStart_BP`
  (params (Anim :type "AnimMontage Object Reference"))
  ;[0.3725 0.3961 1] Виджет оружия и патронов(Надо переделать..)
  ;;[0.3725 0.3961 1] Изменение кол-во патронов при свитче и стрельбе и перезарядки
  (goto _label_4))

(event `self.TrySwitchWeaponBP`
  ;[0.3725 0.3961 1] Виджет оружия и патронов(Надо переделать..)
  ;;[0.3725 0.3961 1] Создание виджетов и изменение иконок при свитчеоружия
  (goto _label_3))

(event `OnStaminaChanged_Event_0` :!signature `self.OnStaminaChanged`
  (params (NewStamina :type "Float (double-precision)"))
  ;[0.3725 0.3961 1] Виджет оружия и патронов(Надо переделать..)
  ;;[0.3725 0.3961 1] Создание виджетов и изменение иконок при свитчеоружия
  (`self.ChangeStaminaWidget` NewStamina))

(event `InputAction|OpenInventory`
  (params (Key :type "Key Structure"))
  (bind _returnvalue (`GameplayStatics.GetPlayerController` 0))
  (bind _returnvalue_2 (`GameplayStatics.GetPlayerController` 0))
  ;[0.3725 0.3961 1] Открытие инвентаря
  (:`Pressed`
    (if (`self.IsInventoryOpened`)
      (set `PlayerController.bShowMouseCursor` false _returnvalue)
      (`WidgetBlueprintLibrary.SetInputMode_GameOnly` _returnvalue)
      (`Widget.RemoveFromParent` (stale _returnvalue_3))
      (set `self.IsInventoryOpened` false)
      (set `self.SlotPosition` (-50.0 -350.0)) ; Setting slot position to default value
      (else
        (bind _returnvalue_3 (`|CreateWidget` "/Game/Blueprint/UI/Inventory/InventoryBase.InventoryBase_C"))
        (`UserWidget.AddToViewport` _returnvalue_3 0)
        (set `self.CanvasPanelOfInventoryBase` (`/Game/Blueprint/UI/Inventory/InventoryBase.CanvasPanel_0` _returnvalue_3))
        (`self.CreateInventorySlots`)
        (set `self.IsInventoryOpened` true)
        (set `self.SlotPosition` (-50.0 -350.0)) ; Setting slot position to default value
        (set `PlayerController.bShowMouseCursor` true _returnvalue_2)
        (`WidgetBlueprintLibrary.SetInputMode_GameAndUIEx` _returnvalue_2 _returnvalue_3)))))

(event `self.CharHealthComponent.OnHealthChange`
  (params (Health :type "Float (single-precision)") (Damage :type "Float (single-precision)"))
  ;[1 0.8667 0.2667] Создание декали и партиклов крови при уроне
  (`self.ChangeHealthWidget`)
  (if (< Damage 0.0)
    (if (> (`KismetMathLibrary.RandomFloat`) 0.6)
      (`GameplayStatics.SpawnDecalAtLocation` (select `int` (`KismetMathLibrary.RandomIntegerInRange` 0 3) :`0` "/Game/LargeFiles/Environment/Decals/M_BloodV1.M_BloodV1" :`1` "/Game/LargeFiles/Environment/Decals/M_BloodV2.M_BloodV2" :`2` "/Game/LargeFiles/Environment/Decals/M_BloodV3.M_BloodV3" :`3` "/Game/LargeFiles/Environment/Decals/M_BloodV4.M_BloodV4" :!type "MaterialInterface Object Reference") (30.0 60.0 60.0) (- (`self.K2_GetActorLocation`) (`KismetMathLibrary.MakeVector` (`KismetMathLibrary.RandomFloatInRange` -40.0 40.0) (`KismetMathLibrary.RandomFloatInRange` -40.0 40.0) 80.0)) (struct :`Pitch` -90.0) 20.0)
      (`NiagaraFunctionLibrary.SpawnSystemAtLocation` "/Game/LargeFiles/Environment/FX/P_Blood.P_Blood" (- (`self.K2_GetActorLocation`) (`KismetMathLibrary.MakeVector` (`KismetMathLibrary.RandomFloatInRange` 40.0 -40.0) (`KismetMathLibrary.RandomFloatInRange` -10.0 -10.0) (`KismetMathLibrary.RandomFloatInRange` -10.0 -10.0)))))))

(event `InputAction|SprintChangeInput`
  (params (Key :type "Key Structure"))
  ;[0.3291 1 0.398] Состояния передвижения
  (:`Pressed`
    (set `self.IsSprintRunEnabled` true)
    (`self.ChangeMovementState` :!label _label_5))
  (:`Released`
    (set `self.IsSprintRunEnabled` false)
    (goto _label_5)))

(event `InputAction|WalkChangeInput`
  (params (Key :type "Key Structure"))
  ;[0.3291 1 0.398] Состояния передвижения
  (:`Pressed`
    (set `self.IsWalkEnabled` true)
    (goto _label_5))
  (:`Released`
    (set `self.IsWalkEnabled` false)
    (goto _label_5)))

(event `InputAction|AimChangeInput`
  (params (Key :type "Key Structure"))
  ;[0.3291 1 0.398] Состояния передвижения
  (:`Pressed`
    (set `self.IsAimEnabled` true)
    (goto _label_5))
  (:`Released`
    (set `self.IsAimEnabled` false)
    (goto _label_5)))

(event `Key|N`
  (params (Key :type "Key Structure"))
  (bind _topdowncameracomponent (`self.TopDownCameraComponent`))
  ;[1 0.8667 0.2667] Night VIsion
  (:`Pressed`
    (`GameplayStatics.SpawnSound2D` "/Game/PostProcess/NightVision/NightVision_Cue.NightVision_Cue" 1.0 1.0 0.0 null)
    (`/Engine/EditorBlueprintResources/StandardMacros.FlipFlop`
      (:`A`
        (`CameraComponent.SetPostProcessBlendWeight` _topdowncameracomponent 1.0)
        (bind _returnvalue (`GameplayStatics.GetActorOfClass` "/Script/Engine.DirectionalLight"))
        (`LightComponentBase.SetCastShadows` (`Light.LightComponent` _returnvalue) false))
      (:`B`
        (`CameraComponent.SetPostProcessBlendWeight` _topdowncameracomponent 0.0)
        (bind _returnvalue_2 (`GameplayStatics.GetActorOfClass` "/Script/Engine.DirectionalLight"))
        (`LightComponentBase.SetCastShadows` (`Light.LightComponent` _returnvalue_2) true)))))

(event `self.CharHealthComponent.OnShieldChange`
  (params (Shield :type "Float (single-precision)") (Damage :type "Float (single-precision)"))
  ;[1 0.8667 0.2667] Спавн партиклов искр при нанесении урона щиту
  (`self.ChangeShieldWidget`)
  (if (< Damage 0.0)
    (`NiagaraFunctionLibrary.SpawnSystemAtLocation` "/Game/LargeFiles/Environment/FX/P_Sparks2.P_Sparks2" (+ (`self.K2_GetActorLocation`) (`KismetMathLibrary.MakeVector` (`KismetMathLibrary.RandomFloatInRange` 10.0 -10.0) (`KismetMathLibrary.RandomFloatInRange` 10.0 20.0) (`KismetMathLibrary.RandomFloatInRange` 20.0 40.0))) (`KismetMathLibrary.MakeRotator` 0.0))))

(fn `CameraShakeFunction`
  (`GameplayStatics.PlayWorldCameraShake` "/Game/Blueprint/Game/BP_CameraShake.BP_CameraShake_C" (`SceneComponent.K2_GetComponentLocation` (`self.TopDownCameraComponent`)) 300.0 30.0))

(fn `CameraSldeFunction`
  (params (A :type "Float (double-precision)"))
  (bind _camerachangedistance (`self.CameraChangeDistance`))
  (bind _targetarmlength (`SpringArmComponent.TargetArmLength` (`self.CameraBoom`)))
  (if (`self.SlideDone`)
    (if (!= A 0.0)
      (if (> 0.0 A)
        (if (> (`self.CameraHeightMax`) (+ _targetarmlength _camerachangedistance))
          (set `self.SlideUp` true)
          (set `self.SlideDone` true :!label _label)
          (bind _returnvalue (`KismetSystemLibrary.K2_SetTimer` null "SlideTimeFunction" (`self.TimerStep`) true))
          (set `self.SlideTImer` _returnvalue))
        (elif (> (- _targetarmlength _camerachangedistance) (`self.CameraHeightMin`))
          (set `self.SlideUp` false)
          (goto _label))))))

(fn `ChangeAmmoWidget`
  (params (self2 :type "TextBlock Object Reference") (self3 :type "/Game/Blueprint/UI/Inventory/ProjectileWidget Object Reference"))
  (bind _returnvalue (`self.GetCurrentWeapon`))
  (bind _returnvalue_2 (`WeaponDefault.GetWeaponRound` _returnvalue))
  (`TextBlock.SetText` self2 (`KismetTextLibrary.Conv_IntToText` _returnvalue_2))
  (bind (_weaponsetting_weaponclass _weaponsetting_rateoffire _weaponsetting_reloadtime _weaponsetting_maxround) (break `WeaponInfo` (`WeaponDefault.WeaponSetting` _returnvalue)))
  (`/Game/Blueprint/UI/Inventory/ProjectileWidget.ChangeProgressBar` self3 _weaponsetting_maxround _returnvalue_2))

(fn `ChangeHealthWidget`
  (bind _returnvalue (`TPSHealthComponent.GetCurrentHealth` (`self.CharHealthComponent`)))
  (`/Game/Blueprint/UI/HealthWidget.HealthChange` (`self.HealthWidget`) _returnvalue 0.0))

(fn `ChangeShieldWidget`
  (bind _returnvalue (`TPSCharacterHealthComponent.GetCurrentShield` (`self.CharHealthComponent`)))
  (`/Game/Blueprint/UI/HealthWidget.ShieldChange` (`self.HealthWidget`) _returnvalue 0.0))

(fn `ChangeStaminaWidget`
  (params (CurrentStamina :type "Float (double-precision)"))
  (`/Game/Blueprint/UI/StaminaWidget.ChangeStaminaProgressBar` (`self.StaminaWidget`) CurrentStamina))

(fn `CreateInventorySlots`
  (locals (IteratorLines :type Integer) (iteratorRows :type Integer) (Slot :type "/Game/Blueprint/UI/Inventory/InventorySlot Object Reference"))
  (bind (_slotposition_x _slotposition_y) (`KismetMathLibrary.BreakVector2D` (`self.SlotPosition`)))
  (bind _slot (`local.Slot`))
  (bind _slot_2 (`local.Slot`))
  (bind (_slotposition_x_2 _slotposition_y_2) (`KismetMathLibrary.BreakVector2D` (`self.SlotPosition`)))
  (bind (_slotposition_x_3 _slotposition_y_3) (`KismetMathLibrary.BreakVector2D` (`self.SlotPosition`)))
  (bind _iconofslot (`/Game/Blueprint/UI/Inventory/InventorySlot.IconOfSlot` (`local.Slot`)))
  (bind _ammoslots (`InventoryComponent.AmmoSlots` (`self.InventoryComponent`)))
  (bind _output_nameitem (break `WeaponSlot` (`|GetArrayItem` (`InventoryComponent.WeaponSlots` (`self.InventoryComponent`)) (`local.IteratorLines`))))
  ;[1 1 1] Creating a row
  (for _index (range 5)
    (set `local.iteratorRows` _index)
    (set `self.SlotPosition` (`KismetMathLibrary.MakeVector2D` _slotposition_x_2 (+ _slotposition_y_2 120.0)))
    ;[1 1 1] Creating a line
    (for _index_2 (range 5)
      (set `local.IteratorLines` _index_2)
      (bind _returnvalue (`|CreateWidget` "/Game/Blueprint/UI/Inventory/InventorySlot.InventorySlot_C"))
      (bind _output_get (set `local.Slot` _returnvalue))
      (bind _returnvalue_2 (`CanvasPanel.AddChildToCanvas` (`self.CanvasPanelOfInventoryBase`) _output_get))
      (bind _output_get_2 (set `self.SlotPosition` (`KismetMathLibrary.MakeVector2D` (+ _slotposition_x 75.0) _slotposition_y)))
      (`CanvasPanelSlot.SetPosition` _returnvalue_2 _output_get_2)
      ;[1 1 1] Setting Slot Icon depends on row number 1 - Weapon 2 - Projectiles 3 - idk(smt in future) 4 - idk
      (switch `int` (`local.iteratorRows`)
        (:`1`
          _)
        (:`2`
          _))
      (if (< (`KismetArrayLibrary.Array_Length` (`InventoryComponent.WeaponSlots` (`self.InventoryComponent`))) (+ (`local.IteratorLines`) 1))
        (`Image.SetBrushFromTexture` (`/Game/Blueprint/UI/Inventory/InventorySlot.IconOfSlot` _slot_2) "/Game/Blueprint/UI/Inventory/EmptyIcon.EmptyIcon" false)
        (else
          (bind _asbp_game_instance (cast `/Game/Blueprint/Game/BP_GameInstance` (`GameplayStatics.GetGameInstance`)))
          (bind _outinfo (`TPSGameInstance.GetWeaponInfoByName` _asbp_game_instance _output_nameitem))
          (set `/Game/Blueprint/UI/Inventory/InventorySlot.Info` (make `WeaponInfo` null (`.RateOfFire` (break `WeaponInfo` _outinfo)) (`.ReloadTime` (break `WeaponInfo` _outinfo)) (`.MaxRound` (break `WeaponInfo` _outinfo)) 1 (`.DispersionWeapon` (break `WeaponInfo` _outinfo)) null null null (`.ProjectileSetting` (break `WeaponInfo` _outinfo)) (`.WeaponDamage` (break `WeaponInfo` _outinfo)) (`.DistacneTrace` (break `WeaponInfo` _outinfo))) _slot_2)
          (if (== (`local.iteratorRows`) 1)
            (`Image.SetBrushFromTexture` _iconofslot (`.WeaponIcon` (break `WeaponInfo` _outinfo)) false)
            (set `/Game/Blueprint/UI/Inventory/InventorySlot.id` 1 (`local.Slot`))
            (elif (< (`KismetArrayLibrary.Array_Length` _ammoslots) 0)
              (`Image.SetBrushFromTexture` _iconofslot "/Game/Blueprint/UI/Inventory/EmptyIcon.EmptyIcon" false)
              (else
                (for _array_element _ammoslots
                  (if (`|EnumEquality` (break `AmmoSlot` _array_element) (`.WeaponType` (break `WeaponInfo` _outinfo)))
                    (`self.SetAmmoSlots` (`/Game/Blueprint/UI/Inventory/InventorySlot.AmmoCout` _slot) _iconofslot (`.ProjectileIcon` (break `WeaponInfo` _outinfo)) (`.Cout` (break `AmmoSlot` _array_element)))
                    (set `/Game/Blueprint/UI/Inventory/InventorySlot.id` 2 _slot)))))))))
    (set `self.SlotPosition` (`KismetMathLibrary.MakeVector2D` -50.0 _slotposition_y_3)) ; -50 is default value of AxisX
  ))

(fn `HealthWidgetCreating`
  (bind _returnvalue (`|CreateWidget` "/Game/Blueprint/UI/HealthWidget.HealthWidget_C"))
  (`UserWidget.AddToViewport` _returnvalue 0)
  (set `self.HealthWidget` _returnvalue)
  (bind _returnvalue_2 (`|CreateWidget` "/Game/Blueprint/UI/StaminaWidget.StaminaWidget_C"))
  (`UserWidget.AddToViewport` _returnvalue_2 0)
  (set `self.StaminaWidget` _returnvalue_2)
  (bind _asbp_game_state_base (cast `/Game/Blueprint/Game/BP_GameStateBase` (`GameplayStatics.GetGameState`)))
  (bind _currentlives (`/Game/Blueprint/Game/BP_GameStateBase.GetCurrentLives` _asbp_game_state_base))
  (bind _returnvalue_3 (`|CreateWidget` "/Game/Blueprint/UI/UI_StatsWidget.UI_StatsWidget_C"))
  (bind _output_get (set `self.StatsWidget` _returnvalue_3))
  (`UserWidget.AddToViewport` _output_get 0)
  (`/Game/Blueprint/UI/UI_StatsWidget.ChangeLivesWidget` _output_get _currentlives))

(fn `PlayReloadinAnim`
  (`/Game/Blueprint/UI/Inventory/ProjectileWidget.PlayReloadingAnim` (`self.ProjectileWidget`) (`self.CurrentWeaponReloadingTime`)))

(fn `SetAmmoSlots`
  (params (Text :type "TextBlock Object Reference") (SlotsIcon :type "Image Object Reference") (AmmoIcon :type "Texture2D Object Reference") (CurrentCout :type Integer))
  (`Image.SetBrushFromTexture` SlotsIcon AmmoIcon false)
  (`Widget.SetVisibility` Text "Visible")
  (if false
    (`TextBlock.SetText` Text "0")
    (else
      (`TextBlock.SetText` Text (`KismetTextLibrary.Conv_IntToText` CurrentCout)))))

(fn `SlideTimeFunction`
  (bind _cameraboom (`self.CameraBoom`))
  (bind _camerachangedistancestep (`self.CameraChangeDistanceStep`))
  (bind _targetarmlength (`SpringArmComponent.TargetArmLength` _cameraboom))
  (bind _output_get (set `self.CurrentSlideChangeDistance` (+ (`self.CurrentSlideChangeDistance`) _camerachangedistancestep)))
  (set `SpringArmComponent.TargetArmLength` (select `bool` (`self.SlideUp`) :`false` (- _targetarmlength _camerachangedistancestep) :`true` (+ _targetarmlength _camerachangedistancestep)) _cameraboom)
  (if (>= _output_get (`self.CameraChangeDistance`))
    (set `self.CurrentSlideChangeDistance` 0.0)
    (`KismetSystemLibrary.K2_ClearAndInvalidateTimerHandle` (`self.SlideTImer`))))

(fn `UserConstructionScript`
  (bind _cameraboom (`self.CameraBoom`))
  (set `SpringArmComponent.TargetArmLength` (`self.Height`) _cameraboom)
  (`SceneComponent.K2_SetRelativeRotation` _cameraboom (`self.CameraRotator`) false false)
  (set `SpringArmComponent.bEnableCameraLag` (`self.Flow`) _cameraboom)
  (set `SpringArmComponent.CameraLagSpeed` (`self.SmoothCoef`) _cameraboom))