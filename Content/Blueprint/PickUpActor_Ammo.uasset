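; Ammo pickup actor, a child of a pickup base class, that gives ammo to a character that overlaps it.
; On OverlapCharacter it runs the parent logic, then asks the character's InventoryComponent whether it can take ammo of the configured weapon type.
; If so, it changes that ammo slot by the pickup's count.
; The PickUp function and construction script only call the parent.
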(event `self.OverlapCharacter`
  (params (InventoryComponent :type "InventoryComponent Object Reference"))
  (`parent.OverlapCharacter` InventoryComponent)
  (bind _returnvalue (`InventoryComponent.CheckCanTakeAmmo` InventoryComponent (`self.WeaponTypeAmmo`)))
  (if _returnvalue
    (`InventoryComponent.AmmoSlotChangeValue` InventoryComponent (`self.WeaponTypeAmmo`) (`self.Cout`))))

(fn `PickUp`
  (`parent.PickUp`))

(fn `UserConstructionScript`
  (`parent.UserConstructionScript`))