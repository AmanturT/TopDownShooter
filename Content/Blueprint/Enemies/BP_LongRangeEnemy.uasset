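; Long-range enemy Blueprint that keeps track of nearby hideout locations and can pick one at random.
; PlayerTrigger overlap events add actors tagged "Hideout" to a map of object name to location, and remove them when overlap ends.
; GetRandomHideout returns a random location from that map.
; The construction script and walk-speed update only call the parent class.
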(event `self.PlayerTrigger.OnComponentBeginOverlap`
  (params (OverlappedComponent :type "PrimitiveComponent Object Reference") (OtherActor :type "Actor Object Reference") (OtherComp :type "PrimitiveComponent Object Reference") (OtherBodyIndex :type Integer) (bFromSweep :type Boolean) (SweepResult :type "HitResult Structure (by ref)"))
  (if (`self.ActorHasTag` OtherActor "Hideout")
    (`BlueprintMapLibrary.Map_Add` (`self.HideoutsLocations`) (`KismetSystemLibrary.GetObjectName` OtherActor) (`self.K2_GetActorLocation` OtherActor))))

(event `self.PlayerTrigger.OnComponentEndOverlap`
  (params (OverlappedComponent :type "PrimitiveComponent Object Reference") (OtherActor :type "Actor Object Reference") (OtherComp :type "PrimitiveComponent Object Reference") (OtherBodyIndex :type Integer))
  (if (`self.ActorHasTag` OtherActor "Hideout")
    (`BlueprintMapLibrary.Map_Remove` (`self.HideoutsLocations`) (`KismetSystemLibrary.GetObjectName` OtherActor))))

(fn `GetRandom Hideout`
  (returns (HideoutLocation :type "Vector Structure"))
  (bind _values (`BlueprintMapLibrary.Map_Values` (`self.HideoutsLocations`)))
  (return (`KismetArrayLibrary.Array_Random` _values)))

(fn `UpdateWalkSpeed`
  (params (NewSpeed :type "Float (double-precision)"))
  (`parent.UpdateWalkSpeed` NewSpeed))

(fn `UserConstructionScript`
  (`parent.UserConstructionScript`))