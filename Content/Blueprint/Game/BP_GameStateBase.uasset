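; Base Game State Blueprint that tracks the player's lives for respawning.
; CanRespawnPlayer spends one life and allows a respawn while CurrentLives is above zero.
; When none remain, it refuses the respawn, resets CurrentLives to MaxLives and reports zero lives.
; GetCurrentLives exposes the count, and the event graph holds no active logic.
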(fn `CanRespawnPlayer`
  (returns (bCanRespawn :type Boolean) (CurrentLives :type Integer))
  (if (> (`self.CurrentLives`) 0)
    (bind _output_get (set `self.CurrentLives` (- (`self.CurrentLives`) 1)))
    (return true _output_get)
    (else
      (set `self.CurrentLives` (`self.MaxLives`))
      (return false 0))))

(fn `GetCurrentLives`
  (returns (CurrentLives :type Integer))
  (return (`self.CurrentLives`)))

(fn `UserConstructionScript`)