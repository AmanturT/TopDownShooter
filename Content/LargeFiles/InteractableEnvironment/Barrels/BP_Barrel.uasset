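; BP_Barrel is an interactable environment barrel that explodes when another actor overlaps it.
; Any actor overlap calls PlayExplosion, which destroys the Barrel component, then spawns the explosion particle effect and sound at its former location.
; A scale coefficient sizes the effect; no damage is applied, and the actor itself is not destroyed.
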(event `self.ReceiveActorBeginOverlap`
  (params (OtherActor :type "Actor Object Reference"))
  (`self.PlayExplosion`))

(fn `PlayExplosion`
  (bind _barrel (`self.Barrel`))
  (bind _returnvalue (* (`self.CoefOfExplosionScale`) 1.0))
  (bind _output_get (set `self.BarrelLocation` (`SceneComponent.K2_GetComponentLocation` _barrel)))
  (`ActorComponent.K2_DestroyComponent` _barrel)
  (`GameplayStatics.SpawnEmitterAtLocation` "/Game/LargeFiles/Environment/FX/Particles/P_Explosion.P_Explosion" _output_get (struct) (`KismetMathLibrary.MakeVector` _returnvalue _returnvalue _returnvalue))
  (`GameplayStatics.PlaySoundAtLocation` "/Game/LargeFiles/Environment/FX/Audio/Cues/Explosion_Cue.Explosion_Cue" (`self.BarrelLocation`) (struct) 1.0 1.0 0.0 null null null))

(fn `UserConstructionScript`)