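; Base enemy Blueprint that takes damage, shows damage numbers and awards points when killed.
; AnyDamage passes negated damage to the TPSHealth component, whose health-change and death events are bound on BeginPlay.
; Each health change spawns a DisplayDamageActor at a slightly randomized offset, initialized with damage and current health.
; On death it adds PointsForKill to BP_GameStateBase and destroys itself, provided the game state cast succeeds.
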(event `self.ReceiveBeginPlay`
  (bind _tpshealth (`self.TPSHealth`))
  (add `TPSHealthComponent.OnHealthChange` _tpshealth (delegate `OnHealthChange_Event`))
  (add `TPSHealthComponent.OnDead` _tpshealth (delegate `OnDeadEvent`)))

(event `OnHealthChange_Event`
  (params (Health :type "Float (double-precision)") (Damage :type "Float (double-precision)"))
  (bind _returnvalue (`|SpawnActorFromClass` "/Game/Blueprint/DisplayDamageActor.DisplayDamageActor_C" (`KismetMathLibrary.MakeTransform` (+ (`self.K2_GetActorLocation`) (+ (`self.LocalPointsHealthNumber`) (`KismetMathLibrary.MakeVector` (`KismetMathLibrary.RandomFloatInRange` -10.0 10.0) (`KismetMathLibrary.RandomFloatInRange` -10.0 10.0))))) "Undefined" "OverrideRootScale" null null))
  (`/Game/Blueprint/DisplayDamageActor.Init Actor` _returnvalue Damage Health))

(event `OnDeadEvent`
  (bind _asbp_game_state_base (cast `/Game/Blueprint/Game/BP_GameStateBase` (`GameplayStatics.GetGameState`)))
  (`/Game/Blueprint/Game/BP_GameStateBase.AddPoints` _asbp_game_state_base (`self.PointsForKill`))
  (`self.K2_DestroyActor`))

(event `self.ReceiveAnyDamage`
  (params (Damage :type "Float (single-precision)") (DamageType :type "DamageType Object Reference") (InstigatedBy :type "Controller Object Reference") (DamageCauser :type "Actor Object Reference"))
  (`TPSHealthComponent.ChangeHealthValue` (`self.TPSHealth`) (* Damage -1.0)))

(fn `UserConstructionScript`)